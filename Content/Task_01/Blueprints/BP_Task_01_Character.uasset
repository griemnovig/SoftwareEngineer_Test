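; Player character for Task 01 that finds interactable actors under the crosshair and interacts with them.
; A camera-forward trace finds the aimed point, then a second trace from the character toward it, limited to InteractDistance, returns the hit actor.
; Every tick, actors implementing BPI_Interact are told to show their interact label.
; The IA_Interact input sends them the interact message.
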(event `self.ReceiveTick`
  (params (DeltaSeconds :type "Float (single-precision)"))
  (`self.TryToShowInteractLabel`))

(event `EnhancedInput|/Game/Basic/Input/IA_Interact`
  (params (ActionValue :type Boolean) (ElapsedSeconds :type "Float (double-precision)") (TriggeredSeconds :type "Float (double-precision)") (InputAction :type "InputAction Object Reference" :default "/Game/Basic/Input/IA_Interact.IA_Interact"))
  (:`Triggered`
    (`self.TryToInteract`)))

(fn `GetActorFromTraceThrowCrosshair`
  (returns (TargetActor :type "Actor Object Reference"))
  (bind _returnvalue (`self.K2_GetActorLocation`))
  (bind _returnvalue_2 (`SceneComponent.K2_GetComponentLocation` (`self.Camera`)))
  (bind (_outhit _returnvalue_3) (`KismetSystemLibrary.LineTraceSingle` :`Start` _returnvalue_2 :`End` (+ _returnvalue_2 (* (`KismetMathLibrary.GetForwardVector` (`SceneComponent.K2_GetComponentRotation` (`self.Camera`))) 1500)) :`TraceChannel` "TraceTypeQuery1" :`DrawTime` 0.5))
  (if _returnvalue_3
    (bind _outhit_2 (`KismetSystemLibrary.LineTraceSingle` :`Start` _returnvalue :`End` (+ _returnvalue (* (`KismetMathLibrary.Normal` (- (`.ImpactPoint` (`GameplayStatics.BreakHitResult` _outhit)) (`self.K2_GetActorLocation`))) (`self.InteractDistance`))) :`TraceChannel` "TraceTypeQuery1" :`DrawTime` 1.0))
    (bind (_bblockinghit _binitialoverlap _time _distance _location _impactpoint _normal _impactnormal _physmat _hitactor) (`GameplayStatics.BreakHitResult` _outhit_2))
    (if _bblockinghit
      (return _hitactor)
      (else
        (return null)))
    (else
      (return null))))

(fn `TryToInteract`
  (bind _targetactor (`self.GetActorFromTraceThrowCrosshair`))
  (`/Engine/EditorBlueprintResources/StandardMacros.IsValid` _targetactor
    (:`Is Valid`
      (if (`KismetSystemLibrary.DoesImplementInterface` _targetactor "/Game/Task_01/Blueprints/BPI_Interact.BPI_Interact_C")
        (message `/Game/Task_01/Blueprints/BPI_Interact.MakeInteract` _targetactor)))))

(fn `TryToShowInteractLabel`
  (bind _targetactor (`self.GetActorFromTraceThrowCrosshair`))
  (`/Engine/EditorBlueprintResources/StandardMacros.IsValid` _targetactor
    (:`Is Valid`
      (if (`KismetSystemLibrary.DoesImplementInterface` _targetactor "/Game/Task_01/Blueprints/BPI_Interact.BPI_Interact_C")
        (message `/Game/Task_01/Blueprints/BPI_Interact.ShowInteractLabel` _targetactor)))))

(fn `UserConstructionScript`)