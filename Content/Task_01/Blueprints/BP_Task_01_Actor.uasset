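; Interactable task actor that swaps its sphere material on interact, shows a label with a hide timer, and drives a screen-space marker widget.
; Tick projects the actor's location to screen, hiding the marker when projection fails and showing distance text when on-screen.
; Off-screen markers clamp to the viewport edge and scale by how far outside they are.
; A FadeDistance-sized collision sphere plays or reverses a timeline on overlap to fade marker opacity.
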(event `/Game/Task_01/Blueprints/BPI_Interact.MakeInteract`
  ;[1 1 1] Interact interface
  (`PrimitiveComponent.SetMaterial` (`self.Sphere`) 0 (`self.InteractReplaceMaterial`)))

(event `/Game/Task_01/Blueprints/BPI_Interact.ShowInteractLabel`
  ;[1 1 1] Interact interface
  (`KismetSystemLibrary.K2_SetTimerDelegate` (`|CreateDelegate` :!event `HideIntercatLabel`) (`self.TimeToHideInteractLabel`))
  (`SceneComponent.SetHiddenInGame` (`self.InteractLabelWidget`) false false))

(event `self.ReceiveTick`
  (params (DeltaSeconds :type "Float (single-precision)"))
  (bind _returnvalue (`GameplayStatics.GetPlayerController` 0))
  (bind (_screenposition _returnvalue_2) (`GameplayStatics.ProjectWorldToScreen` _returnvalue (`self.K2_GetActorLocation`) true))
  ;[1 1 1] Rendering marker widget
  (`/Engine/EditorBlueprintResources/StandardMacros.IsValid` (`GameplayStatics.GetPlayerCharacter` 0)
    (:`Is Valid`
      (`/Engine/EditorBlueprintResources/StandardMacros.IsValid` _returnvalue
        (:`Is Valid`
          (set `self.MarkerPositionOnScreen` _screenposition)
          (bind _output_get (set `self.bWidgetCanSee` _returnvalue_2))
          (`Widget.SetVisibility` (`self.MarkerWidgetRef`) (select `bool` _output_get :`false` "Collapsed" :`true` "Visible" :!type "ESlateVisibility Enum"))
          (if (`self.bWidgetCanSee`)
            (`self.RenderingMarkerWidget`)))))))

(event `self.ReceiveBeginPlay`
  (`self.InitWidgets`))

(event `self.FadeWidgetCollision.OnComponentBeginOverlap`
  (params (OverlappedComponent :type "PrimitiveComponent Object Reference") (OtherActor :type "Actor Object Reference") (OtherComp :type "PrimitiveComponent Object Reference") (OtherBodyIndex :type Integer) (bFromSweep :type Boolean) (SweepResult :type "HitResult Structure (by ref)"))
  ;[1 1 1] Fade in/out
  (bind (_direction _opacity) (`Timeline|FadeIn/OutTimeLine` :!label _label)
    (:`Update`
      (`Widget.SetRenderOpacity` (`self.MarkerWidgetRef`) _opacity))))

(event `self.FadeWidgetCollision.OnComponentEndOverlap`
  (params (OverlappedComponent :type "PrimitiveComponent Object Reference") (OtherActor :type "Actor Object Reference") (OtherComp :type "PrimitiveComponent Object Reference") (OtherBodyIndex :type Integer))
  ;[1 1 1] Fade in/out
  (goto _label :!via `Reverse`))

(fn `CalculateOutOfScreenWidgetPosition`
  (returns (ViewportPosition :type "Vector2D Structure"))
  (locals (lClampMinX :type "Float (double-precision)") (lClampMinY :type "Float (double-precision)") (lDesiredWidgetSize :type "Vector2D Structure"))
  (bind _markerpositiononscreen_x (`KismetMathLibrary.BreakVector2D` (`self.MarkerPositionOnScreen`)))
  (bind (_markerpositiononscreen_x_2 _markerpositiononscreen_y) (`KismetMathLibrary.BreakVector2D` (`self.MarkerPositionOnScreen`)))
  (bind (_x _y) (`KismetMathLibrary.BreakVector2D` (`WidgetLayoutLibrary.GetViewportSize`)))
  (bind _output_get (set `local.lDesiredWidgetSize` (`Widget.GetDesiredSize` (`self.MarkerWidgetRef`))))
  (set `local.lClampMinX` (/ (`KismetMathLibrary.BreakVector2D` _output_get) 2.0))
  (set `local.lClampMinY` (/ (`.Y` (`KismetMathLibrary.BreakVector2D` _output_get)) 2.0))
  (return (`KismetMathLibrary.MakeVector2D` (`KismetMathLibrary.FClamp` _markerpositiononscreen_x (`local.lClampMinX`) (- _x (`local.lClampMinX`))) (`KismetMathLibrary.FClamp` _markerpositiononscreen_y (`local.lClampMinY`) (- _y (`local.lClampMinY`))))))

(fn `CalculateWidgetScale`
  (params (bWidgetOnScreen :type Boolean))
  (locals (lScaleValue :type "Float (double-precision)" :default 0.0) (lViewportSize :type "Vector2D Structure") (lXValue :type "Float (double-precision)") (lYValue :type "Float (double-precision)"))
  (bind _markerpositiononscreen_x (`KismetMathLibrary.BreakVector2D` (`self.MarkerPositionOnScreen`)))
  (bind (_markerpositiononscreen_x_2 _markerpositiononscreen_y) (`KismetMathLibrary.BreakVector2D` (`self.MarkerPositionOnScreen`)))
  (bind (_lviewportsize_x _lviewportsize_y) (`KismetMathLibrary.BreakVector2D` (`local.lViewportSize`)))
  (bind _markerpositiononscreen_x_3 (`KismetMathLibrary.BreakVector2D` (`self.MarkerPositionOnScreen`)))
  (bind _lviewportsize_x_2 (`KismetMathLibrary.BreakVector2D` (`local.lViewportSize`)))
  (bind _markerpositiononscreen_x_4 (`KismetMathLibrary.BreakVector2D` (`self.MarkerPositionOnScreen`)))
  (bind (_markerpositiononscreen_x_5 _markerpositiononscreen_y_2) (`KismetMathLibrary.BreakVector2D` (`self.MarkerPositionOnScreen`)))
  (bind (_markerpositiononscreen_x_6 _markerpositiononscreen_y_3) (`KismetMathLibrary.BreakVector2D` (`self.MarkerPositionOnScreen`)))
  (if bWidgetOnScreen
    (`Widget.SetRenderScale` (`self.MarkerWidgetRef`) (1.0 1.0))
    (else
      (set `local.lViewportSize` (`WidgetLayoutLibrary.GetViewportSize`))
      (set `local.lXValue` (`KismetMathLibrary.Abs` (`KismetMathLibrary.SelectFloat` _markerpositiononscreen_x_3 (`KismetMathLibrary.FMax` (- _markerpositiononscreen_x_4 _lviewportsize_x_2)) (< _markerpositiononscreen_x 0.0))))
      (set `local.lYValue` (`KismetMathLibrary.Abs` (`KismetMathLibrary.SelectFloat` _markerpositiononscreen_y_3 (`KismetMathLibrary.FMax` (- _markerpositiononscreen_y _lviewportsize_y)) (< _markerpositiononscreen_y_2 0.0))))
      (bind _output_get (set `local.lScaleValue` (`KismetMathLibrary.MapRangeClamped` (`KismetMathLibrary.FMax` (`local.lXValue`) (`local.lYValue`)) (`self.StartScaleDecreaseDistance`) (`self.EndScaleDecreaseDistance`) 1.0 (`self.MaxScaleDecreaseValue`))))
      (`Widget.SetRenderScale` (`self.MarkerWidgetRef`) (`KismetMathLibrary.MakeVector2D` _output_get _output_get)))))

(fn `HideIntercatLabel`
  (`SceneComponent.SetHiddenInGame` (`self.InteractLabelWidget`) true false))

(fn `InitWidgets`
  (`|ExecutionSequence`
    (:`then_0`
      (bind _returnvalue (`|CreateWidget` "/Game/Task_01/Widgets/W_Marker.W_Marker_C" (`GameplayStatics.GetPlayerController` 0)))
      (bind _output_get (set `self.MarkerWidgetRef` _returnvalue))
      (`Widget.SetVisibility` _output_get "Collapsed")
      (`UserWidget.AddToPlayerScreen` _output_get 0))
    (:`then_1`
      (`SphereComponent.SetSphereRadius` (`self.FadeWidgetCollision`) (`self.FadeDistance`) true))))

(fn `IsWidgetOnScreen`
  (returns (Value :type Boolean))
  (bind (_returnvalue_x _returnvalue_y) (`KismetMathLibrary.BreakVector2D` (`WidgetLayoutLibrary.GetViewportSize`)))
  (bind (_markerpositiononscreen_x _markerpositiononscreen_y) (`KismetMathLibrary.BreakVector2D` (`self.MarkerPositionOnScreen`)))
  (bind (_markerpositiononscreen_x_2 _markerpositiononscreen_y_2) (`KismetMathLibrary.BreakVector2D` (`self.MarkerPositionOnScreen`)))
  (return (and (< _markerpositiononscreen_x_2 _returnvalue_x) (< _markerpositiononscreen_y_2 _returnvalue_y) (> _markerpositiononscreen_x 0.0) (> _markerpositiononscreen_y 0.0))))

(fn `RenderingMarkerWidget`
  (bind _value (`self.IsWidgetOnScreen`))
  (`self.CalculateWidgetScale` _value)
  (`/Game/Task_01/Widgets/W_Marker.SetTextDistance` (`self.MarkerWidgetRef`) (select `bool` _value :`true` (`|FormatText` "{Distance} m" (`KismetMathLibrary.Round` (/ (`self.GetDistanceTo` (`GameplayStatics.GetPlayerCharacter` 0)) 100.0)))))
  (`UserWidget.SetPositionInViewport` (`self.MarkerWidgetRef`) (select `bool` _value :`false` (`self.CalculateOutOfScreenWidgetPosition`) :`true` (`self.MarkerPositionOnScreen`)) true))

(fn `UserConstructionScript`)