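; Player character that rides the BP_Trajectory spline and throws physics balls with a predicted landing marker.
; A timeline moves it along the spline, with play rate set from the spline's loop time, which speed-up and slow-down inputs adjust.
; Holding shoot maps camera pitch to launch speed along actor forward and moves a BP_HitPlace marker to the traced impact.
; Release spawns a BP_PhysicBall with that velocity.
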(event `self.ReceiveBeginPlay`
  (bind _returnvalue (`GameplayStatics.GetActorOfClass` "/Game/Task_05/BP_Trajectory.BP_Trajectory_C"))
  (set `self.SplineRef` _returnvalue)
  (bind _splineref (`self.SplineRef`)
    (:`then`
      (`self.K2_SetActorLocation` (`/Game/Task_05/BP_Trajectory.GetStartPointLocation` _splineref) false true)
      (`self.StartMoveOnSpline`))
    (:`else`)))

(event `EnhancedInput|/Game/Basic/Input/IA_SplineSpeedUp`
  (params (ActionValue :type Boolean) (ElapsedSeconds :type "Float (double-precision)") (TriggeredSeconds :type "Float (double-precision)") (InputAction :type "InputAction Object Reference" :default "/Game/Basic/Input/IA_SplineSpeedUp.IA_SplineSpeedUp"))
  ;[1 1 1] Move on spline
  (:`Triggered`
    (`self.SetSplineCompleteTime` (`/Game/Task_05/BP_Trajectory.TryToUpCompleteTime` (`self.SplineRef`)))))

(event `EnhancedInput|/Game/Basic/Input/IA_SplineSpeedDown`
  (params (ActionValue :type Boolean) (ElapsedSeconds :type "Float (double-precision)") (TriggeredSeconds :type "Float (double-precision)") (InputAction :type "InputAction Object Reference" :default "/Game/Basic/Input/IA_SplineSpeedDown.IA_SplineSpeedDown"))
  ;[1 1 1] Move on spline
  (:`Triggered`
    (`self.SetSplineCompleteTime` (`/Game/Task_05/BP_Trajectory.TryToDownCompleteTime` (`self.SplineRef`)))))

(event `StartMoveOnSpline`
  ;[1 1 1] Move on spline
  (`self.SetSplineCompleteTime` (`/Game/Task_05/BP_Trajectory.GetTimeToCompleteLoop` (`self.SplineRef`)))
  (bind (_direction _movetrack) (`Timeline|SplineTimeline`)
    (:`Update`
      (`self.MovingOnSpline` _movetrack))))

(event `EnhancedInput|/Game/Basic/Input/IA_Shoot`
  (params (ActionValue :type Boolean) (ElapsedSeconds :type "Float (double-precision)") (TriggeredSeconds :type "Float (double-precision)") (InputAction :type "InputAction Object Reference" :default "/Game/Basic/Input/IA_Shoot.IA_Shoot"))
  ;[1 1 1] Shoot
  (:`Started`
    (`self.SpawnPredictHitPlace`))
  (:`Ongoing`
    (bind _hirresult (`self.PredictProjectilePath`))
    (`self.MovePredictHitPlace` _hirresult))
  (:`Completed`
    (`self.SpawnPhysicsBall`)
    (set `self.HitPlaceRef` null)))

(fn `MovePredictHitPlace`
  (params (Hit :type "HitResult Structure (by ref)"))
  (bind _hitplaceref (`self.HitPlaceRef`)
    (:`then`
      (`self.K2_SetActorLocation` _hitplaceref (`.ImpactPoint` (`GameplayStatics.BreakHitResult` Hit)) false true))
    (:`else`)))

(fn `MovingOnSpline`
  (params (Alpha :type "Float (double-precision)"))
  (`self.K2_SetActorLocation` (+ (`SplineComponent.GetLocationAtDistanceAlongSpline` (`/Game/Task_05/BP_Trajectory.Spline` (`self.SplineRef`)) (`KismetMathLibrary.Lerp` 0.0 (`SplineComponent.GetSplineLength` (`/Game/Task_05/BP_Trajectory.Spline` (`self.SplineRef`))) Alpha) "World") (0.0 0.0 100.0))))

(fn `PredictProjectilePath`
  (returns (HirResult :type "HitResult Structure"))
  (bind (_returnvalue_roll _returnvalue_pitch) (`KismetMathLibrary.BreakRotator` (`SceneComponent.K2_GetComponentRotation` (`self.Camera`))))
  (bind _output_get (set `self.InitialProjectileVelocity` (* (`self.GetActorForwardVector`) (`KismetMathLibrary.MapRangeClamped` _returnvalue_pitch (* (`self.ThrowAngle`) -1.0) (`self.ThrowAngle`) (`self.MinThrowDistance`) (`self.MaxThrowDistance`)))))
  (bind _outhit (`GameplayStatics.Blueprint_PredictProjectilePath_ByTraceChannel` (`self.K2_GetActorLocation`) _output_get true 15.0 "ECC_WorldDynamic" false (`|MakeArray` self :!type "Actor Object Reference") "ForOneFrame" 0.0 10.0))
  (return _outhit))

(fn `SetSplineCompleteTime`
  (params (`TimeToCompeteLoop(InSec)` :type "Float (double-precision)"))
  (`TimelineComponent.SetPlayRate` (`self.SplineTimeline`) (/ 1.0 `TimeToCompeteLoop(InSec)`)))

(fn `SpawnPhysicsBall`
  (bind _returnvalue (`|SpawnActorFromClass` "/Game/Task_05/BP_PhysicBall.BP_PhysicBall_C" (`KismetMathLibrary.MakeTransform` (`self.K2_GetActorLocation`)) "AlwaysSpawn" "MultiplyWithRoot" null null))
  (`PrimitiveComponent.AddImpulse` (`/Game/Task_05/BP_PhysicBall.Sphere` _returnvalue) (`self.InitialProjectileVelocity`) "None" true))

(fn `SpawnPredictHitPlace`
  (bind _returnvalue (`|SpawnActorFromClass` "/Game/Task_05/BP_HitPlace.BP_HitPlace_C" (`KismetMathLibrary.MakeTransform` (0.0 0.0 -100.0)) "AlwaysSpawn" "MultiplyWithRoot" null null))
  (set `self.HitPlaceRef` _returnvalue))

(fn `UserConstructionScript`)