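; BP_Trajectory is a spline-based path that exposes its start point and loop completion time to other code.
; GetStartPointLocation returns the first spline point in world space, and GetTimeToCompleteLoop returns the current loop time in seconds.
; TryToUpCompleteTime shortens that time by one second and TryToDownCompleteTime lengthens it, both clamped between minimum and maximum limits.
; It only holds data, with no movement logic of its own.
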(fn `GetStartPointLocation`
  (returns (Location :type "Vector Structure"))
  (return (`SplineComponent.GetLocationAtSplinePoint` (`self.Spline`) 0 "World")))

(fn `GetTimeToCompleteLoop`
  (returns (`Time(InSec)` :type "Float (double-precision)"))
  (return (`self.TimeToCompleteLoop(InSec)`)))

(fn `TryToDownCompleteTime`
  (returns (NewTime :type "Float (double-precision)"))
  (bind _output_get (set `self.TimeToCompleteLoop(InSec)` (`KismetMathLibrary.FClamp` (+ (`self.TimeToCompleteLoop(InSec)`) 1.0) (`self.MinCompleteTime`) (`self.MaxCompleteTime`))))
  (return _output_get))

(fn `TryToUpCompleteTime`
  (returns (NewTime :type "Float (double-precision)"))
  (bind _output_get (set `self.TimeToCompleteLoop(InSec)` (`KismetMathLibrary.FClamp` (- (`self.TimeToCompleteLoop(InSec)`) 1.0) (`self.MinCompleteTime`) (`self.MaxCompleteTime`))))
  (return _output_get))

(fn `UserConstructionScript`)