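; Task 04 character Blueprint, apparently a test bed for verifying replication of a dynamic component and an object's values.
; BeginPlay calls the parent, then adds a WBP_ReplicationVerify widget to the viewport for its player controller.
; CreateDynamicComp adds and stores a skeletal mesh component, while ChangeValueEvent randomizes ReplicatedObj's bool, float and int.
; Tick prints the component's name and the object's values whenever each is valid.
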(event `self.ReceiveBeginPlay`
  (`parent.ReceiveBeginPlay`)
  (bind _asplayer_controller (cast `PlayerController` (`self.GetController`)))
  (bind _returnvalue (`|CreateWidget` "/Game/Task_04/WBP_ReplicationVerify.WBP_ReplicationVerify_C" _asplayer_controller))
  (`UserWidget.AddToViewport` _returnvalue 0))

(event `self.ReceiveTick`
  (params (DeltaSeconds :type "Float (single-precision)"))
  (`|ExecutionSequence`
    (:`then_0`
      (bind _skeletalmeshcomp (`self.SkeletalMeshComp`)
        (:`then`
          (`KismetSystemLibrary.PrintString` (`KismetSystemLibrary.GetDisplayName` _skeletalmeshcomp) true true (struct :`G` 0.66 :`B` 1.0 :`A` 1.0) 0.0))
        (:`else`)))
    (:`then_1`
      (bind _replicatedobj (`self.ReplicatedObj`)
        (:`then`
          (`KismetSystemLibrary.PrintString` (`KismetStringLibrary.Concat_StrStr` (`KismetStringLibrary.Conv_BoolToString` (`UReplicateObject.boolvalue` _replicatedobj)) "      " (`KismetStringLibrary.Conv_DoubleToString` (`UReplicateObject.floatvalue` _replicatedobj)) "      " (`KismetStringLibrary.Conv_IntToString` (`UReplicateObject.intvalue` _replicatedobj))) true true (struct :`G` 0.66 :`B` 1.0 :`A` 1.0) 0.0))
        (:`else`)))))

(event `CreateDynamicComp`
  (bind _returnvalue (`AddComponent|NODE_AddSkeletalMeshComponent-1`))
  (set `self.SkeletalMeshComp` _returnvalue))

(event `ChangeValueEvent`
  (`self.ChangeValues`))

(fn `ChangeValues`
  (bind _replicatedobj (`self.ReplicatedObj`)
    (:`then`
      (set `UReplicateObject.boolvalue` (`KismetMathLibrary.RandomBool`) _replicatedobj)
      (set `UReplicateObject.floatvalue` (`KismetMathLibrary.RandomFloat`) _replicatedobj)
      (set `UReplicateObject.intvalue` (`KismetMathLibrary.RandomInteger` 0) _replicatedobj))
    (:`else`)))

(fn `UserConstructionScript`)