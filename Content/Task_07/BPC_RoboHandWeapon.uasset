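; Robo-hand weapon component that fires a cable-tethered hook to grab objects and carry them in front of its owner.
; InitiateRoboHand spawns the hook and cable; a hit disables the struck component's physics and attaches its actor to the hook.
; ControlRoboHand drives projectile velocity forward until max range, or after a grab eases toward an aim-adjusted point at the grab distance.
; FinishRoboHand restores physics and destroys both spawned actors.
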(fn `ControlRoboHand`
  (`self.RoboHookRef`
    (:`then`
      (if (`self.bExistGrabbedObject`)
        (`self.SetGrabbedObjDesirableLoc`)
        (`self.SetVelocityHookAfterGrab`)
        (`self.SetHookRotation`)
        (else
          (`self.SetVelocityHookBeforeGrab`)
          (if (>= (`self.GetDistanceToPlayer`) (`self.MaxHookDistance`))
            (`self.FinishRoboHand`)))))
    (:`else`)))

(fn `FinishRoboHand`
  (`|ExecutionSequence`
    (:`then_0`
      (bind _grabbedcomp (`self.GrabbedComp`)
        (:`then`
          (`PrimitiveComponent.SetSimulatePhysics` _grabbedcomp true))
        (:`else`)))
    (:`then_1`
      (bind _cableref (`self.CableRef`)
        (:`then`
          (`Actor.K2_DestroyActor` _cableref))
        (:`else`)))
    (:`then_2`
      (bind _robohookref (`self.RoboHookRef`)
        (:`then`
          (remove `Actor.OnActorHit` _robohookref (`|CreateDelegate` :!event `OnHitObject`))
          (`Actor.K2_DestroyActor` _robohookref))
        (:`else`)))
    (:`then_3`
      (set `self.bExistGrabbedObject` false))))

(fn `GetDistanceFromHookToDesirableLoc`
  (returns (ReturnValue :type "Float (double-precision)"))
  (return (`KismetMathLibrary.VSize` (- (`self.GrabbedObjDesirableLocation`) (`Actor.K2_GetActorLocation` (`self.RoboHookRef`))))))

(fn `GetDistanceToPlayer`
  (returns (ReturnValue :type "Float (single-precision)"))
  (bind _robohookref (`self.RoboHookRef`)
    (:`then`
      (return (`Actor.GetDistanceTo` _robohookref (`self.GetOwner`))))
    (:`else`)))

(fn `InitiateRoboHand`
  (bind _returnvalue (`self.GetOwner`))
  (bind _returnvalue_2 (`|SpawnActorFromClass` "/Game/Task_07/BP_RoboHook.BP_RoboHook_C" (`KismetMathLibrary.MakeTransform` (+ (`Actor.K2_GetActorLocation` _returnvalue) (* (`Actor.GetActorForwardVector` _returnvalue) 65) (0.0 0.0 20.0)) (`.OutRotation` (`Actor.GetActorEyesViewPoint` _returnvalue))) "AlwaysSpawn" "MultiplyWithRoot" (`self.GetOwner`) null))
  (bind _output_get (set `self.RoboHookRef` _returnvalue_2))
  (add `Actor.OnActorHit` _output_get (`|CreateDelegate` :!event `OnHitObject`))
  (bind _returnvalue_3 (`|SpawnActorFromClass` "/Game/Task_07/BP_CableActor.BP_CableActor_C" (`KismetMathLibrary.MakeTransform` (`Actor.K2_GetActorLocation` (`self.GetOwner`))) "AlwaysSpawn" "MultiplyWithRoot" (`self.GetOwner`) null))
  (bind _output_get_2 (set `self.CableRef` _returnvalue_3))
  (`Actor.K2_AttachToActor` _output_get_2 (`self.GetOwner`) "None" "SnapToTarget" "KeepWorld" "KeepWorld" true)
  (`CableComponent.SetAttachEndTo` (`CableActor.CableComponent` (`self.CableRef`)) (`self.RoboHookRef`) "None" "None"))

(fn `OnHitObject`
  (params (SelfActor :type "Actor Object Reference") (OtherActor :type "Actor Object Reference") (NormalImpulse :type "Vector Structure") (Hit :type "HitResult Structure (by ref)"))
  (if (not (`self.bExistGrabbedObject`))
    (`self.RoboHookRef`
      (:`then`
        (bind _output_get (set `self.GrabbedComp` (`.HitComponent` (`GameplayStatics.BreakHitResult` Hit))))
        (`PrimitiveComponent.SetSimulatePhysics` _output_get false)
        (bind _output_get_2 (set `self.GrabbedObject` (`local.OtherActor`)))
        (bind _returnvalue (`Actor.K2_AttachToActor` _output_get_2 (`self.RoboHookRef`) "None" "SnapToTarget" "KeepWorld" "KeepWorld" false))
        (set `self.bExistGrabbedObject` _returnvalue)
        (set `self.DistanceToHookedObject` (`self.GetDistanceToPlayer`))
        (return))
      (:`else`))))

(fn `SetGrabbedObjDesirableLoc`
  (bind _returnvalue (`self.GetOwner`))
  (bind (_returnvalue_x _returnvalue_y _returnvalue_z) (`KismetMathLibrary.BreakVector` (* (`KismetMathLibrary.GetForwardVector` (`.OutRotation` (`Actor.GetActorEyesViewPoint` (`self.GetOwner`)))) 1500.0)))
  (set `self.GrabbedObjDesirableLocation` (+ (+ (`Actor.K2_GetActorLocation` _returnvalue) (* (`Actor.GetActorForwardVector` _returnvalue) (`self.DistanceToHookedObject`))) (`KismetMathLibrary.MakeVector` 0.0 0.0 (`KismetMathLibrary.FMax` _returnvalue_z))))
  (return))

(fn `SetHookRotation`
  (`Actor.K2_SetActorRotation` (`self.RoboHookRef`) (`KismetMathLibrary.FindLookAtRotation` (`Actor.K2_GetActorLocation` (`self.GetOwner`)) (`Actor.K2_GetActorLocation` (`self.RoboHookRef`))) false))

(fn `SetVelocityHookAfterGrab`
  (set `MovementComponent.Velocity` (* (`KismetMathLibrary.Normal` (- (`self.GrabbedObjDesirableLocation`) (`Actor.K2_GetActorLocation` (`self.RoboHookRef`)))) (* (`self.GetDistanceFromHookToDesirableLoc`) 2.0)) (`/Game/Task_07/BP_RoboHook.ProjectileMovement` (`self.RoboHookRef`))))

(fn `SetVelocityHookBeforeGrab`
  (bind (_returnvalue_x _returnvalue_y _returnvalue_z) (`KismetMathLibrary.BreakVector` (`Actor.GetActorForwardVector` (`self.RoboHookRef`))))
  (set `MovementComponent.Velocity` (* (`KismetMathLibrary.MakeVector` _returnvalue_x _returnvalue_y (`KismetMathLibrary.FMax` _returnvalue_z -0.03)) (`self.MaxHookSpeed`)) (`/Game/Task_07/BP_RoboHook.ProjectileMovement` (`self.RoboHookRef`))))