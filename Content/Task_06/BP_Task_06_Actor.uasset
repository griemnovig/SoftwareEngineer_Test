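; Actor that wanders around the BP_Task_06_Target actor using steering behavior.
; It seeks a random point near the target, picking a new one when close enough.
; Each tick, forward motion plus a steering vector toward that point sets ProjectileMovement velocity, and rotation follows velocity.
; A short forward capsule trace detects blocking hits, which zero velocity and randomize rotation to escape obstacles.
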(event `self.ReceiveBeginPlay`
  (bind _returnvalue (`GameplayStatics.GetActorOfClass` "/Game/Task_06/BP_Task_06_Target.BP_Task_06_Target_C"))
  (set `self.TargetRef` _returnvalue)
  (`self.SetNewRandomTargetLocation`))

(event `self.ReceiveTick`
  (params (DeltaSeconds :type "Float (single-precision)"))
  (bind _selflocation (`self.SelfLocation`))
  (if (`self.IsEnoughDistanceToChangeTargetLocation`)
    (`self.SetNewRandomTargetLocation`))
  (set `self.SelfLocation` (`self.K2_GetActorLocation`))
  (set `self.DesirableDirection` (`self.GetDisarableDirection`))
  (set `self.CurrentForwardVector` (`self.GetActorForwardVector`))
  (set `self.SteeringDirection` (`self.GetSteeringDirection`))
  (bind _outhit (`KismetSystemLibrary.CapsuleTraceSingle` _selflocation (+ _selflocation (* (`self.CurrentForwardVector`) 50.0)) 20.0 20.0 "TraceTypeQuery1" false (`|MakeArray` self :!type "Actor Object Reference") "None" true (struct :`R` 1.0 :`A` 1.0) (struct :`G` 1.0 :`A` 1.0) 0.1))
  (if (`GameplayStatics.BreakHitResult` _outhit)
    (set `MovementComponent.Velocity` (0.0 0.0 0.0) (`self.ProjectileMovement`))
    (`self.K2_SetActorRotation` (`KismetMathLibrary.RandomRotator` true))
    (else
      (set `MovementComponent.Velocity` (`self.GetCurrentVelocity`) (`self.ProjectileMovement`))
      (`self.K2_SetActorRotation` (`KismetMathLibrary.MakeRotFromX` (`MovementComponent.Velocity` (`self.ProjectileMovement`)))))))

(fn `GetCurrentVelocity`
  (returns (ReturnValue :type "Vector Structure"))
  (return (+ (* (`self.CurrentForwardVector`) (`self.Speed`)) (* (`self.SteeringDirection`) (`self.SteeringMultiplier`)))))

(fn `GetDisarableDirection`
  (returns (ReturnValue :type "Vector Structure"))
  (locals (lNormalizedVector :type "Vector Structure" :default (0.0 0.0 0.0)))
  (bind _returnvalue (- (`self.NearbyTargetLocation`) (`self.SelfLocation`)))
  (bind _output_get (set `local.lNormalizedVector` (`KismetMathLibrary.Normal` _returnvalue)))
  (if (`KismetMathLibrary.Vector_IsZero` _output_get)
    (return (`KismetMathLibrary.GreaterGreater_VectorRotator` _returnvalue (struct :`Yaw` 2.0)))
    (else
      (return (`local.lNormalizedVector`)))))

(fn `GetSteeringDirection`
  (returns (ReturnValue :type "Vector Structure"))
  (return (`KismetMathLibrary.Normal` (- (`self.DesirableDirection`) (`self.CurrentForwardVector`)))))

(fn `IsEnoughDistanceToChangeTargetLocation`
  (returns (ReturnValue :type Boolean))
  (return (<= (`KismetMathLibrary.VSize` (- (`self.NearbyTargetLocation`) (`self.SelfLocation`))) (`self.DistanceToChangeTargetLocation`))))

(fn `SetNewRandomTargetLocation`
  (locals (lTargetLocation :type "Vector Structure" :default (0.0 0.0 0.0)))
  (bind _deviationintargetlocation (`self.DeviationInTargetLocation`))
  (bind _returnvalue (`KismetMathLibrary.RandomFloatInRange` (* _deviationintargetlocation -1.0) _deviationintargetlocation))
  (bind _targetref (`self.TargetRef`)
    (:`then`
      (bind _output_get (set `local.lTargetLocation` (`self.K2_GetActorLocation` _targetref)))
      (set `self.NearbyTargetLocation` (`KismetMathLibrary.MakeVector` (+ (.x _output_get) _returnvalue) (+ (.y _output_get) _returnvalue) (+ (.z _output_get) _returnvalue))))
    (:`else`)))

(fn `UserConstructionScript`)